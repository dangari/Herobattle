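; Player controller that lets the player place command flags for three heroes, one all-hero flag or three single flags.
; Hotkeys select a flag, Tick previews it under the cursor via trace, and left-click commits it or otherwise forwards to the character.
; Placement replaces the old flag and updates hero state, though every single flag targets hero 0 with the all-flag's location.
; Pressing a hotkey during selection cancels, destroying flags and resetting hero states.
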(event Custom|OnUseFlag
  (params (SelectedFlag :type SelectedFlag%20Enum))
  ;[1 1 1] Handels Flag inputs
  (CallFunction|DeActivateFlag SelectedFlag))

(event EventBeginPlay
  ;[1 1 1] On Game Start
  (bind _asthird_person_character (Utilities|Casting|CastToThirdPersonCharacter (Game|GetPlayerCharacter 0)))
  (Variables|Default|SetCurrentCharacter _asthird_person_character))

(event EventTick
  (params (DeltaSeconds :type Float%20%28single-precision%29))
  ;[1 1 1] Handels Flag movement
  (if (Utilities|Enum|NotEqual(Enum) (Variables|Flags|GetCurrentSelectedFlag) "NONE")
    (CallFunction|UpdateSelectedFlag)))

(event Input|ActionEvents|InputActionFlagTwo
  (params (Key :type Key%20Structure :default "AnyKey"))
  ;[1 1 1] Handels Flag inputs
  (:Pressed
    (CallFunction|OnUseFlag "FLAGG_TWO")))

(event Input|ActionEvents|InputActionFlagThree
  (params (Key :type Key%20Structure :default "AnyKey"))
  ;[1 1 1] Handels Flag inputs
  (:Pressed
    (CallFunction|OnUseFlag "FLAGG_THREE")))

(event Input|ActionEvents|InputActionFlagAll
  (params (Key :type Key%20Structure :default "AnyKey"))
  ;[1 1 1] Handels Flag inputs
  (:Pressed
    (CallFunction|OnUseFlag "FLAGALL")))

(event Input|ActionEvents|InputActionFlagOne
  (params (Key :type Key%20Structure :default "AnyKey"))
  ;[1 1 1] Handels Flag inputs
  (:Pressed
    (CallFunction|OnUseFlag "FLAGG_ONE")))

(event Input|MouseEvents|LeftMouseButton
  (params (Key :type Key%20Structure :default "AnyKey"))
  ;[1 1 1] Left Mouse Button
  (:Pressed
    (if (Utilities|Enum|NotEqual(Enum) (Variables|Flags|GetCurrentSelectedFlag) "NONE")
      (CallFunction|PlaceFlagonClickedLocation)
      (else
        (bind _asthird_person_character (Utilities|Casting|CastToThirdPersonCharacter (Pawn|GetControlledPawn)))
        (Default|LeftMousButtonClicked _asthird_person_character)))))

(fn ConstructionScript)

(fn ActivateFlag
  (params (NewParam :type SelectedFlag%20Enum))
  (switch Utilities|FlowControl|Switch|SwitchonSelectedFlag NewParam))

(fn SpawnFlagatMouse)

(fn UpdateSelectedFlag
  (bind (_hitresult _returnvalue) (Game|Player|GetHitResultUnderCursorbyChannel "TraceTypeQuery3" true))
  (bind _location (Collision|BreakHitResult _hitresult))
  (bind _returnvalue_2 (Math|Transform|MakeTransform _location "0, 0, 0" "1,1.000000,1"))
  (if _returnvalue
    (if (!= (Variables|Flags|GetTempFlag) 0)
      (Transformation|SetActorTransform (Variables|Flags|GetTempFlag) _returnvalue_2)
      (else
        (bind _returnvalue_3 (Game|SpawnActorfromClass "/Game/Blueprints/Flag.Flag_C" _returnvalue_2 "Undefined" 0 0))
        (Variables|Flags|SetTempFlag _returnvalue_3))))
  (return))

(fn DeActivateFlag
  (params (FlagType :type SelectedFlag%20Enum))
  (if (Utilities|Enum|Equal(Enum) (Variables|Flags|GetCurrentSelectedFlag) "NONE")
    (Variables|Flags|SetCurrentSelectedFlag FlagType)
    (else
      (CallFunction|DestroyFlag FlagType)
      (if (!= (Variables|Flags|GetTempFlag) 0)
        (Actor|DestroyActor (Variables|Flags|GetTempFlag))
        (Variables|Flags|SetTempFlag 0)
        (CallFunction|SetHeroState)
        (Variables|Flags|SetCurrentSelectedFlag "NONE")))))

(fn PlaceFlag
  (bind (_hitresult _returnvalue) (Game|Player|GetHitResultUnderCursorbyChannel "TraceTypeQuery3" true))
  (bind _location (Collision|BreakHitResult _hitresult))
  (bind _returnvalue_2 (Math|Transform|MakeTransform _location))
  (Variables|Default|SetleftMouseClicked true)
  (if _returnvalue
    (if (!= (Variables|/Game/ThirdPerson/Blueprints/ThirdPersonCharacter.ThirdPersonCharacter_C|GetFlaggAll (Variables|Default|GetCurrentCharacter)) 0)
      (Transformation|SetActorTransform (Variables|/Game/ThirdPerson/Blueprints/ThirdPersonCharacter.ThirdPersonCharacter_C|GetFlaggAll (Variables|Default|GetCurrentCharacter)) _returnvalue_2)
      (else
        (bind _returnvalue_3 (Game|SpawnActorfromClass "/Game/Blueprints/Flag.Flag_C" _returnvalue_2 "Undefined" 0 0))))
    (Variables|Flags|SetCurrentSelectedFlag "NONE")
    (Variables|/Game/ThirdPerson/Blueprints/ThirdPersonCharacter.ThirdPersonCharacter_C|SetFlaggAll (Variables|Default|GetCurrentCharacter) _returnvalue_3))
  (return))

(fn PlaceFlagonClickedLocation
  (bind (_hitresult _returnvalue) (Game|Player|GetHitResultUnderCursorbyChannel "TraceTypeQuery3" true))
  (bind _currentselectedflag (Variables|Flags|GetCurrentSelectedFlag))
  (if _returnvalue
    (Transformation|SetActorLocation (Variables|Flags|GetTempFlag) (.Location (Collision|BreakHitResult _hitresult)) false false)
    (switch Utilities|FlowControl|Switch|SwitchonSelectedFlag (Variables|Flags|GetCurrentSelectedFlag)
      (:FLAGALL
        (CallFunction|SetNewFlag _currentselectedflag (Variables|Flags|GetFlagALLRef)))
      (:FLAGG_ONE
        (CallFunction|SetNewFlag _currentselectedflag (Variables|Flags|GetFlag1Ref)))
      (:FLAGG_TWO
        (CallFunction|SetNewFlag _currentselectedflag (Variables|Flags|GetFlag2Ref)))
      (:FLAGG_THREE
        (CallFunction|SetNewFlag _currentselectedflag (Variables|Flags|GetFlag3Ref))))))

(fn SetNewFlag
  (params (FlagRef :type SelectedFlag%20Enum) (Flag :type Flag%20Object%20Reference))
  (LocalVariables|SetTempCurrentSelectedFlag FlagRef)
  (if (!= Flag 0)
    (CallFunction|DestroyFlag (LocalVariables|GetTempCurrentSelectedFlag)))
  (switch Utilities|FlowControl|Switch|SwitchonSelectedFlag (LocalVariables|GetTempCurrentSelectedFlag)
    (:FLAGALL
      (Variables|Flags|SetFlagALLRef (Variables|Flags|GetTempFlag))
      (CallFunction|SetAllFlagtoHeroes))
    (:FLAGG_ONE
      (Variables|Flags|SetFlag1Ref (Variables|Flags|GetTempFlag))
      (CallFunction|SetSingleFlagPosition "FLAGSINGEL"))
    (:FLAGG_TWO
      (Variables|Flags|SetFlag2Ref (Variables|Flags|GetTempFlag))
      (CallFunction|SetSingleFlagPosition "FLAGSINGEL"))
    (:FLAGG_THREE
      (Variables|Flags|SetFlag3Ref (Variables|Flags|GetTempFlag))
      (CallFunction|SetSingleFlagPosition "FLAGSINGEL")))
  (Variables|Flags|SetTempFlag 0)
  (Variables|Flags|SetCurrentSelectedFlag "NONE"))

(fn DestroyFlag
  (params (Selected%20Flag :type SelectedFlag%20Enum))
  (switch Utilities|FlowControl|Switch|SwitchonSelectedFlag Selected%20Flag
    (:FLAGALL
      (CallFunction|CheckandDestroyFlag (Variables|Flags|GetFlagALLRef))
      (Variables|Flags|SetFlagALLRef 0))
    (:FLAGG_ONE
      (CallFunction|CheckandDestroyFlag (Variables|Flags|GetFlag1Ref))
      (Variables|Flags|SetFlag1Ref 0))
    (:FLAGG_TWO
      (CallFunction|CheckandDestroyFlag (Variables|Flags|GetFlag2Ref))
      (Variables|Flags|SetFlag2Ref 0))
    (:FLAGG_THREE
      (CallFunction|CheckandDestroyFlag (Variables|Flags|GetFlag3Ref))
      (Variables|Flags|SetFlag3Ref 0))))

(fn CheckandDestroyFlag
  (params (Flag :type Flag%20Object%20Reference))
  (if (!= Flag 0)
    (Actor|DestroyActor Flag))
  (return))

(fn SetAllFlagtoHeroes
  (bind _asherobattle_character (Utilities|Casting|CastToHerobattleCharacter (Pawn|GetControlledPawn)))
  (for _index (range 0 2)
    (bind _returnvalue (Class|HerobattleCharacter|GetHero _asherobattle_character (Math|Conversions|ToByte(Integer) _index)))
    (Variables|/Script/Herobattle.HeroBattleHero|SetallFlagVectorLocation _returnvalue (Transformation|GetActorLocation (Variables|Flags|GetFlagALLRef)))
    (Variables|/Script/Herobattle.HeroBattleHero|SetcurrentState _returnvalue "FLAGALL")))

(fn SetSingleFlagPosition
  (params (HeroState :type HeroState%20Enum) (Index :type Byte))
  (bind _asherobattle_character (Utilities|Casting|CastToHerobattleCharacter (Pawn|GetControlledPawn)))
  (bind _returnvalue (Class|HerobattleCharacter|GetHero _asherobattle_character Index))
  (Variables|/Script/Herobattle.HeroBattleHero|SetallFlagVectorLocation _returnvalue (Transformation|GetActorLocation (Variables|Flags|GetFlagALLRef)))
  (Variables|/Script/Herobattle.HeroBattleHero|SetcurrentState _returnvalue HeroState))

(fn SetHeroState
  (switch Utilities|FlowControl|Switch|SwitchonSelectedFlag (Variables|Flags|GetCurrentSelectedFlag)
    (:FLAGALL
      (CallFunction|SetHeroStateOfAllHeroesNone))
    (:FLAGG_ONE
      (CallFunction|SetHeroStateforSingleFlag :!label _label))
    (:FLAGG_TWO
      (goto _label))
    (:FLAGG_THREE
      (goto _label))))

(fn SetHeroStateforSingleFlag
  (bind _asherobattle_character (Utilities|Casting|CastToHerobattleCharacter (Pawn|GetControlledPawn)))
  (LocalVariables|SetTempCharacter _asherobattle_character)
  (switch Utilities|FlowControl|Switch|SwitchonSelectedFlag (Variables|Flags|GetCurrentSelectedFlag)
    (:FLAGG_ONE
      (CallFunction|UpdateHeroStateSingleFlag (LocalVariables|GetTempCharacter)))
    (:FLAGG_TWO
      (CallFunction|UpdateHeroStateSingleFlag (LocalVariables|GetTempCharacter) 1))
    (:FLAGG_THREE
      (CallFunction|UpdateHeroStateSingleFlag (LocalVariables|GetTempCharacter) 2))))

(fn UpdateHeroStateSingleFlag
  (params (Character :type Herobattle%20Character%20Object%20Reference) (Index :type Byte))
  (bind _returnvalue (Class|HerobattleCharacter|GetHero Character Index))
  (if (!= (Variables|Flags|GetFlagALLRef) 0)
    (Variables|/Script/Herobattle.HeroBattleHero|SetcurrentState _returnvalue "FLAGALL")
    (else
      (Variables|/Script/Herobattle.HeroBattleHero|SetcurrentState _returnvalue "NONE")))
  (return))

(fn SetHeroStateOfAllHeroesNone
  (bind _asherobattle_character (Utilities|Casting|CastToHerobattleCharacter (Pawn|GetControlledPawn)))
  (for _index (range 0 2)
    (bind _returnvalue (Class|HerobattleCharacter|GetHero _asherobattle_character (Math|Conversions|ToByte(Integer) _index)))
    (Variables|/Script/Herobattle.HeroBattleHero|SetcurrentState _returnvalue "NONE")
    (CallFunction|DestroyAllFlags)))

(fn DestroyAllFlags
  (if (!= (Variables|Flags|GetFlagALLRef) 0)
    (Actor|DestroyActor (Variables|Flags|GetFlagALLRef))
    (Variables|Flags|SetFlagALLRef 0)
    (Actor|DestroyActor (Variables|Flags|GetFlag1Ref) :!label _label)
    (Variables|Flags|SetFlag1Ref 0)
    (Actor|DestroyActor (Variables|Flags|GetFlag2Ref) :!label _label_2)
    (Variables|Flags|SetFlag2Ref 0)
    (Actor|DestroyActor (Variables|Flags|GetFlag3Ref) :!label _label_3)
    (Variables|Flags|SetFlag3Ref 0)
    (Actor|DestroyActor (Variables|Flags|GetTempFlag) :!label _label_4)
    (Variables|Flags|SetTempFlag 0)
    (elif (!= (Variables|Flags|GetFlag1Ref) 0)
      (goto _label)
      (elif (!= (Variables|Flags|GetFlag2Ref) 0)
        (goto _label_2)
        (elif (!= (Variables|Flags|GetFlag3Ref) 0)
          (goto _label_3)
          (elif (!= (Variables|Flags|GetTempFlag) 0)
            (goto _label_4)))))))
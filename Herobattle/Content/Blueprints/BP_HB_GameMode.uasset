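; Game mode Blueprint for HB that seeds debug skill data, handles player login setup and returns characters to spawn points.
; BeginPlay converts each SkillList entry into a name and description record in the HBGameState DebugSkillList.
; PostLogin calls TeamColor on the new player's ThirdPersonCharacter, and FinishedPostLogin calls its AfterPostLogin.
; MovetoSpawnLocation teleports a character to the player start found for its controller.
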(event `self.ReceiveBeginPlay`
  (bind _ashbgame_state (cast `HBGameState` (`GameplayStatics.GetGameState`)))
  (for _array_element (`self.skillList`)
    (bind _returnvalue (`Skill.ToString` _array_element))
    (`KismetArrayLibrary.Array_Add` (`HBGameState.DebugSkillList` _ashbgame_state) (make `DebugSkill` (`Skill.name` _array_element) _returnvalue))))

(event `self.ReceiveTick`
  (params (DeltaSeconds :type "Float (single-precision)")))

(event `self.K2_PostLogin`
  (params (NewPlayer :type "PlayerController Object Reference"))
  (`VisualLoggerKismetLibrary.LogText` "BP")
  (bind _asthird_person_character (cast `/Game/ThirdPerson/Blueprints/ThirdPersonCharacter` (`Controller.K2_GetPawn` NewPlayer)))
  (`/Game/ThirdPerson/Blueprints/ThirdPersonCharacter.TeamColor` _asthird_person_character _asthird_person_character))

(event `self.finishedPostLogin`
  (params (NewPlayer :type "PlayerController Object Reference"))
  (bind _asthird_person_character (cast `/Game/ThirdPerson/Blueprints/ThirdPersonCharacter` (`Controller.K2_GetPawn` NewPlayer)))
  (`/Game/ThirdPerson/Blueprints/ThirdPersonCharacter.AfterPostLogin` _asthird_person_character))

(event `self.moveToSpawnLocation`
  (params (character :type "BaseCharacter Object Reference"))
  (`self.K2_SetActorLocation` character (`self.K2_GetActorLocation` (`self.K2_FindPlayerStart` (`Pawn.GetController` character))) false true))

(fn `UserConstructionScript`)
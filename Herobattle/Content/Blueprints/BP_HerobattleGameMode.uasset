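; Game mode for a hero battle that tracks the selected hero and shows its health on the HUD.
; Every tick, while a selected hero is set, it flags the player as having a character selected.
; If the HUD exists, it also sets the target health bar to the hero's current-to-max health ratio.
; The selection itself is not assigned in this Blueprint.
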(event `self.ReceiveTick`
  (params (DeltaSeconds :type "Float (single-precision)"))
  (bind _hud (`self.HUD`))
  (bind _selectedhero (`self.SelectedHero`))
  (if (!= (`self.SelectedHero`) null)
    (set `/Game/ThirdPerson/Blueprints/ThirdPersonCharacter.CharacterSelected` true (`self.Player`))
    (if (!= _hud null)
      (`ProgressBar.SetPercent` (`/Game/Interface/Player_Hud.targetHealth` _hud) (/ (`BaseCharacter.m_Health` _selectedhero) (`BaseCharacter.m_MaxHealth` _selectedhero))))))

(fn `UserConstructionScript`)
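; Player controller that lets the player place a single "flag all" marker in the world with the mouse and hand it to the player's ThirdPersonCharacter.
; The FlagAll input or FlaggAll event toggles placement mode, during which Tick spawns or moves one reused Flag to the cursor trace hit.
; A left click on a hit locks the flag and assigns it to the character's FlaggAll, while toggling off without clicking destroys it.
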(event `FlaggAll`
  (bind _flagallref (`self.FlagALLRef`))
  ;[1 1 1] Activate Flag ALL
  (set `self.FlagAll` (not (`self.FlagAll`)) :!label _label)
  (if (`self.leftMouseClicked`)
    (set `self.leftMouseClicked` false)
    (elif (!= _flagallref null)
      (`self.K2_DestroyActor` _flagallref)
      (set `self.FlagALLRef` null)
      (set `self.leftMouseClicked` false)
      (set `/Game/ThirdPerson/Blueprints/ThirdPersonCharacter.FlaggAll` null (`self.CurrentCharacter`)))))

(event `InputAction|FlagAll`
  (params (Key :type "Key Structure" :default "AnyKey"))
  ;[1 1 1] Activate Flag ALL
  (:`Pressed`
    (goto _label)))

(event `Key|LeftMouseButton`
  (params (Key :type "Key Structure" :default "AnyKey"))
  (bind (_hitresult _returnvalue) (`self.GetHitResultUnderCursorByChannel` "TraceTypeQuery3"))
  (bind _returnvalue_2 (`KismetMathLibrary.MakeTransform` (`.Location` (`GameplayStatics.BreakHitResult` _hitresult))))
  ;[1 1 1] Left Mouse Button
  (:`Pressed`
    (if (`self.FlagAll`)
      (set `self.leftMouseClicked` true)
      (if _returnvalue
        (if (!= (`self.FlagALLRef`) null)
          (`self.K2_SetActorTransform` (`self.FlagALLRef`) _returnvalue_2 false false)
          (else
            (bind _returnvalue_3 (`|SpawnActorFromClass` "/Game/Blueprints/Flag.Flag_C" _returnvalue_2 "Undefined" "OverrideRootScale"))
            (bind _output_get (set `self.FlagALLRef` _returnvalue_3))))
        (set `self.FlagAll` false)
        (set `/Game/ThirdPerson/Blueprints/ThirdPersonCharacter.FlaggAll` _output_get (`self.CurrentCharacter`))))))

(event `self.ReceiveTick`
  (params (DeltaSeconds :type "Float (single-precision)"))
  (bind (_hitresult _returnvalue) (`self.GetHitResultUnderCursorByChannel` "TraceTypeQuery3"))
  (bind _returnvalue_2 (`KismetMathLibrary.MakeTransform` (`.Location` (`GameplayStatics.BreakHitResult` _hitresult))))
  ;[1 1 1] Handels Flag movement
  (if (`self.FlagAll`)
    (set `/Game/ThirdPerson/Blueprints/ThirdPersonCharacter.FlaggAll` null (`self.CurrentCharacter`))
    (if _returnvalue
      (if (!= (`self.FlagALLRef`) null)
        (`self.K2_SetActorTransform` (`self.FlagALLRef`) _returnvalue_2 false false)
        (else
          (bind _returnvalue_3 (`|SpawnActorFromClass` "/Game/Blueprints/Flag.Flag_C" _returnvalue_2 "Undefined" "OverrideRootScale"))
          (set `self.FlagALLRef` _returnvalue_3))))))

(event `self.ReceiveBeginPlay`
  ;[1 1 1] On Game Start
  (bind _asthird_person_character (cast `/Game/ThirdPerson/Blueprints/ThirdPersonCharacter` (`GameplayStatics.GetPlayerCharacter` 0)))
  (set `self.CurrentCharacter` _asthird_person_character))

(fn `UserConstructionScript`)
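; BP_CapturePoint is a level element that tells the player's HUD when a hero enters or leaves a capture point.
; Begin and end overlap events call CheckIfActorIsplayer, which runs client-side only and looks for a locally controlled BaseCharacter to fetch the HUD_HeroBattle widget.
; That widget receives EnterCapturePoint with this actor, or LeftCapturePoint on exit.
; The Blueprint itself holds no capture progress or ownership logic.
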(event `self.ReceiveActorBeginOverlap`
  (params (OtherActor :type "Actor Object Reference"))
  (bind _hud (`self.CheckIfActorIsplayer` OtherActor))
  (if (!= _hud null)
    (`/Game/Interface/Player_Hud.EnterCapturePoint` _hud self)))

(event `self.ReceiveActorEndOverlap`
  (params (OtherActor :type "Actor Object Reference"))
  (`/Engine/EditorBlueprintResources/ActorMacros.Switch Has Authority`
    (:`Remote`
      (bind _hud (`self.CheckIfActorIsplayer` OtherActor))
      (if (!= _hud null)
        (`/Game/Interface/Player_Hud.LeftCapturePoint` _hud)))))

(fn `CheckIfActorIsplayer`
  (params (Actor :type "Object Object Reference"))
  (returns (Hud :type "/Game/Interface/Player_Hud Object Reference"))
  (`/Engine/EditorBlueprintResources/ActorMacros.Switch Has Authority`
    (:`Remote`
      (bind _asbase_character (cast `BaseCharacter` Actor))
      (bind _returnvalue (`Pawn.GetController` _asbase_character))
      (if (!= _returnvalue null)
        (if (`Controller.IsLocalController` _returnvalue)
          (bind _ashud_hero_battle (cast `/Game/Interface/HUD_HeroBattle` (`PlayerController.GetHUD` (`GameplayStatics.GetPlayerController` 0)))))
        (return (`/Game/Interface/HUD_HeroBattle.Hud` _ashud_hero_battle))))))

(fn `UserConstructionScript`)